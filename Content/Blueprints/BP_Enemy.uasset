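; BP_Enemy is an enemy actor that moves in a straight line and awards score when hit by a projectile.
; Each Tick it applies a swept world offset from its Direction and Speed, scaled by delta time.
; Overlapping a BP_Projectile adds a point through BP_GameMode and destroys the enemy, while overlapping a BP_Wall destroys it without scoring.
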(event EventBeginPlay)

(event Collision|EventActorBeginOverlap
  (params (OtherActor :type Actor%20Object%20Reference))
  (Utilities|Casting|CastToBP_Projectile OtherActor
    (:then
      (bind _asbp_game_mode (Utilities|Casting|CastToBP_GameMode (Game|GetGameMode))
        (:then
          (Default|ChangeScore _asbp_game_mode 1))
        (:CastFailed
          _)))
    (:CastFailed
      (Utilities|Casting|CastToBP_Wall OtherActor)))
  (Actor|DestroyActor))

(event EventTick
  (params (DeltaSeconds :type Float%20%28single-precision%29))
  (Transformation|AddActorWorldOffset (* (* (Variables|Default|GetDirection) (Variables|Default|GetSpeed)) DeltaSeconds) true))

(fn ConstructionScript)