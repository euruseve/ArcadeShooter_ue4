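; BP_EnemySpawner is an actor that spawns a random enemy every two seconds at one of its generated spawn points.
; The construction script loops a DoN node back on itself to add Count sphere components spaced by Offset along local Y, collecting them in Components.
; A looping timer started on BeginPlay picks a random component and spawns a scaled-down base, ammo-bonus, life-bonus or life-lose enemy variant there.
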(event Custom|SpawnEnemy
  (Game|SpawnActorfromClass (Utilities|Select :Index (Math|Random|RandomInteger 4) :Option%200 "/Game/Blueprints/BP_Enemy.BP_Enemy_C" :Option%201 "/Game/Blueprints/BP_Enemy_AmmoBonus.BP_Enemy_AmmoBonus_C" :Option%202 "/Game/Blueprints/BP_Emeny_LifeBonus.BP_Emeny_LifeBonus_C" :Option%203 "/Game/Blueprints/BP_Enemy_LifeLose.BP_Enemy_LifeLose_C") (Math|Transform|MakeTransform (Transformation|GetWorldLocation (.OutItem (Utilities|Array|Random (Variables|Default|GetComponents)))) "0, 0, 0" "0.300000,0.300000,0.300000") "Undefined" 0 0))

(event EventBeginPlay
  (Utilities|Time|SetTimerbyEvent (delegate Custom|SpawnEnemy) 2.0 true))

(event Collision|EventActorBeginOverlap
  (params (OtherActor :type Actor%20Object%20Reference)))

(event EventTick
  (params (DeltaSeconds :type Float%20%28single-precision%29)))

(fn ConstructionScript
  (bind _counter (Utilities|FlowControl|DoN (Variables|Default|GetCount) :!label _label)
    (:Exit
      (bind _returnvalue (AddComponent|AddSphereComponent false (Math|Conversions|ToTransform(Vector) (Math|Vector|MakeVector 0.0 (* _counter (Variables|Default|GetOffset)) 0.0))))
      (Utilities|Array|Add (Variables|Default|GetComponents) _returnvalue)
      (goto _label))))