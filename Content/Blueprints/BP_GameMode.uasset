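; BP_GameMode is the game mode that tracks score and best score and drives the HUD and game-over screen.
; On BeginPlay it creates WBP_Main and loads the best score from the PlayerSlot save, defaulting to zero without one.
; Helper functions push lives, ammo and added score to the HUD, or show WBP_GameOver and pause.
; UpdateBestScore raises the best score in memory only; no save happens here.
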(event EventBeginPlay
  (bind _returnvalue (UserInterface|CreateWidget "/Game/Widgets/WBP_Main.WBP_Main_C"))
  (bind _output_get (Variables|Default|SetMainWidget _returnvalue))
  (UserInterface|Viewport|AddtoViewport _output_get 0)
  (SaveGame|DoesSaveGameExist "PlayerSlot")
  (if true
    (bind _returnvalue_2 (SaveGame|LoadGamefromSlot "PlayerSlot"))
    (bind _asbp_save_game (Utilities|Casting|CastToBP_SaveGame _returnvalue_2))
    (Variables|Default|SetBestScore (Variables|/Game/Blueprints/BP_SaveGame.BP_SaveGame_C|GetSaved_BestScore _asbp_save_game))
    (else
      (Variables|Default|SetBestScore 0))))

(event EventTick
  (params (DeltaSeconds :type Float%20%28single-precision%29)))

(fn ConstructionScript)

(fn AddGameOverWidget
  (bind _returnvalue (UserInterface|CreateWidget "/Game/Widgets/WBP_GameOver.WBP_GameOver_C"))
  (UserInterface|Viewport|AddtoViewport _returnvalue 0)
  (Game|SetGamePaused true))

(fn ChangeLifes
  (Default|UpdateLifes (Variables|Default|GetMainWidget) (Variables|Default|GetLifes)))

(fn ChangeAmmo
  (Default|UpdateAmmo (Variables|Default|GetMainWidget) (Variables|Default|GetAmmo)))

(fn ChangeScore
  (params (AddScore :type Integer))
  (bind _output_get (Variables|Default|SetScore (+ (Variables|Default|GetScore) AddScore)))
  (Default|UpdateScore (Variables|Default|GetMainWidget) _output_get))

(fn UpdateBestScore
  (if (> (Variables|Default|GetScore) (Variables|Default|GetBestScore))
    (Variables|Default|SetBestScore (Variables|Default|GetScore))))