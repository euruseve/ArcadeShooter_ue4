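; BP_Enemy_AmmoBonus is an enemy variant that rewards the player with bonus ammo when a projectile hits it.
; On overlap with a BP_Projectile, it adds a fixed amount to the Ammo held in BP_GameMode and calls ChangeAmmo.
; A Sequence then runs the parent's overlap handling for every overlapping actor, so inherited behavior still applies even when the casts fail.
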(event EventBeginPlay
  (|CallParentFunction) ; This node is disabled and will not be called.\nDrag off pins to build functionality.
)

(event Collision|EventActorBeginOverlap
  (params (OtherActor :type Actor%20Object%20Reference))
  (Utilities|FlowControl|Sequence
    (:then_0
      (Utilities|Casting|CastToBP_Projectile OtherActor)
      (bind _asbp_game_mode (Utilities|Casting|CastToBP_GameMode (Game|GetGameMode)))
      (Variables|/Game/Blueprints/BP_GameMode.BP_GameMode_C|SetAmmo _asbp_game_mode (+ (Variables|/Game/Blueprints/BP_GameMode.BP_GameMode_C|GetAmmo _asbp_game_mode) 10))
      (Default|ChangeAmmo _asbp_game_mode))
    (:then_1
      (|CallParentFunction OtherActor))))

(event EventTick
  (params (DeltaSeconds :type Float%20%28single-precision%29))
  (|CallParentFunction DeltaSeconds) ; This node is disabled and will not be called.\nDrag off pins to build functionality.
)

(fn ConstructionScript
  (|CallParentFunction))