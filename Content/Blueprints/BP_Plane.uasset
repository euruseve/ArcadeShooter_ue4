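; Player-controlled plane that moves along the world X axis and fires projectiles.
; MoveUp and MoveDown axis inputs apply fixed, swept world offsets each frame, without delta-time scaling.
; Fire spawns a scaled-down BP_Projectile at the Sphere component's location, then decrements the ammo held in BP_GameMode and calls ChangeAmmo.
; At zero ammo, firing only prints a "No Ammo" message.
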(event EventBeginPlay
  (bind _asbp_game_mode (Utilities|Casting|CastToBP_GameMode (Game|GetGameMode)))
  (Variables|Default|SetGameMode _asbp_game_mode))

(event Collision|EventActorBeginOverlap
  (params (OtherActor :type Actor%20Object%20Reference)))

(event EventTick
  (params (DeltaSeconds :type Float%20%28single-precision%29)))

(event Input|ActionEvents|InputActionFire
  (params (Key :type Key%20Structure))
  (bind _gamemode (Variables|Default|GetGameMode))
  (:Pressed
    (if (== (Variables|/Game/Blueprints/BP_GameMode.BP_GameMode_C|GetAmmo (Variables|Default|GetGameMode)) 0)
      (Development|PrintString "No Ammo")
      (else
        (Game|SpawnActorfromClass "/Game/Blueprints/BP_Projectile.BP_Projectile_C" (Math|Transform|MakeTransform (Transformation|GetWorldLocation (Variables|Default|GetSphere)) "0, 0, 0" "0.400000,0.400000,0.400000") "Undefined" 0 0)
        (Variables|/Game/Blueprints/BP_GameMode.BP_GameMode_C|SetAmmo _gamemode (- (Variables|/Game/Blueprints/BP_GameMode.BP_GameMode_C|GetAmmo (Variables|Default|GetGameMode)) 1))
        (Default|ChangeAmmo _gamemode)))))

(event Input|AxisEvents|InputAxisMoveUp
  (params (AxisValue :type Float%20%28single-precision%29))
  (if (> AxisValue 0.0)
    (Transformation|AddActorWorldOffset "10.000000, 0, 0" true)))

(event Input|AxisEvents|InputAxisMoveDown
  (params (AxisValue :type Float%20%28single-precision%29))
  (if (< AxisValue 0.0)
    (Transformation|AddActorWorldOffset "-10.000000, 0, 0" true)))

(fn ConstructionScript)