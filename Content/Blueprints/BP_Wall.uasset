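; BP_Wall is a barrier that costs the player a life whenever a BP_Enemy overlaps it.
; On overlap it decrements Lifes on BP_GameMode and refreshes them through ChangeLifes.
; While lives remain, a looping timer nudges the wall along negative X in unit steps until the accumulated offset matches FinallOffset.
; At zero lives it updates the best score, adds the game-over widget and saves that score through BP_SaveGame.
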(event Custom|OffsetWall
  (Transformation|AddActorWorldOffset "-1.000000, 0, 0")
  (bind _output_get (Variables|Default|SetCurrentOffset (+ (Variables|Default|GetCurrentOffset) "1.000000, 0, 0")))
  (if (Math|Vector|Equal(Vector) _output_get (Variables|Default|GetFinallOffset) 0.0001)
    (Utilities|Time|ClearandInvalidateTimerbyHandle (Variables|Default|GetOffsetTimer))
    (Variables|Default|SetCurrentOffset "0, 0, 0")))

(event EventBeginPlay)

(event Collision|EventActorBeginOverlap
  (params (OtherActor :type Actor%20Object%20Reference))
  (Utilities|Casting|CastToBP_Enemy OtherActor)
  (bind _asbp_game_mode (Utilities|Casting|CastToBP_GameMode (Game|GetGameMode)))
  (Variables|Default|SetGameMode_Ref _asbp_game_mode)
  (bind _output_get (Variables|/Game/Blueprints/BP_GameMode.BP_GameMode_C|SetLifes _asbp_game_mode (- (Variables|/Game/Blueprints/BP_GameMode.BP_GameMode_C|GetLifes _asbp_game_mode) 1)))
  (Default|ChangeLifes _asbp_game_mode)
  (if (== _output_get 0)
    (Development|PrintString "Game Over")
    (Default|UpdateBestScore (Variables|Default|GetGameMode_Ref))
    (Default|AddGameOverWidget (Variables|Default|GetGameMode_Ref))
    (bind _returnvalue (SaveGame|CreateSaveGameObject "/Game/Blueprints/BP_SaveGame.BP_SaveGame_C"))
    (Variables|/Game/Blueprints/BP_SaveGame.BP_SaveGame_C|SetSaved_BestScore _returnvalue (Variables|/Game/Blueprints/BP_GameMode.BP_GameMode_C|GetBestScore (Variables|Default|GetGameMode_Ref)))
    (SaveGame|SaveGametoSlot _returnvalue "PlayerSlot")
    (else
      (bind _returnvalue_2 (Utilities|Time|SetTimerbyEvent (delegate Custom|OffsetWall) 0.1 true))
      (Variables|Default|SetOffsetTimer _returnvalue_2))))

(event EventTick
  (params (DeltaSeconds :type Float%20%28single-precision%29)))

(fn ConstructionScript)