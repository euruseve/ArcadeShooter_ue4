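; BP_Wall is a wall actor that destroys any BP_Enemy overlapping it and then shifts itself along world negative X.
; Each such overlap sets a looping timer whose event nudges the wall one unit per tick, without sweep, and accumulates the distance in CurrentOffset.
; When CurrentOffset matches FinallOffset, the timer is cleared and the counter resets for the next hit.
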(event Custom|OffsetWall
  (Transformation|AddActorWorldOffset "-1.000000, 0, 0")
  (bind _output_get (Variables|Default|SetCurrentOffset (+ (Variables|Default|GetCurrentOffset) "1.000000, 0, 0")))
  (if (Math|Vector|Equal(Vector) _output_get (Variables|Default|GetFinallOffset) 0.0001)
    (Utilities|Time|ClearandInvalidateTimerbyHandle (Variables|Default|GetOffsetTimer))
    (Variables|Default|SetCurrentOffset "0, 0, 0")))

(event EventBeginPlay)

(event Collision|EventActorBeginOverlap
  (params (OtherActor :type Actor%20Object%20Reference))
  (bind _asbp_enemy (Utilities|Casting|CastToBP_Enemy OtherActor))
  (Actor|DestroyActor _asbp_enemy)
  (bind _returnvalue (Utilities|Time|SetTimerbyEvent (delegate Custom|OffsetWall) 0.1 true))
  (Variables|Default|SetOffsetTimer _returnvalue))

(event EventTick
  (params (DeltaSeconds :type Float%20%28single-precision%29)))

(fn ConstructionScript)