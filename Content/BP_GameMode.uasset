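; Game mode Blueprint that owns the main on-screen widget and handles the game-over screen.
; On BeginPlay it creates WBP_Main, stores it and adds it to the viewport.
; ChangeLifes and ChangeAmmo push the Lifes and Ammo values into that widget.
; AddGameOverWidget shows WBP_GameOver and pauses the game.
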(event EventBeginPlay
  (bind _returnvalue (UserInterface|CreateWidget "/Game/WBP_Main.WBP_Main_C"))
  (bind _output_get (Variables|Default|SetMainWidget _returnvalue))
  (UserInterface|Viewport|AddtoViewport _output_get 0))

(event EventTick
  (params (DeltaSeconds :type Float%20%28single-precision%29)))

(fn ConstructionScript)

(fn AddGameOverWidget
  (bind _returnvalue (UserInterface|CreateWidget "/Game/WBP_GameOver.WBP_GameOver_C"))
  (UserInterface|Viewport|AddtoViewport _returnvalue 0)
  (Game|SetGamePaused true))

(fn ChangeLifes
  (Default|UpdateLifes (Variables|Default|GetMainWidget) (Variables|Default|GetLifes)))

(fn ChangeAmmo
  (Default|UpdateAmmo (Variables|Default|GetMainWidget) (Variables|Default|GetAmmo)))