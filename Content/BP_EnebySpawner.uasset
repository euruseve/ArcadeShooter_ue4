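; Enemy spawner actor that repeatedly spawns BP_Enemy at one of several points laid out in a line.
; The construction script loops a DoN node back into itself to add Count sphere components spaced by Offset along local Y, storing them in Components.
; From BeginPlay, a looping one-second timer spawns a scaled-down enemy at the world location of a randomly picked sphere.
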(event Custom|SpawnEnemy
  (Game|SpawnActorfromClass "/Game/BP_Enemy.BP_Enemy_C" (Math|Transform|MakeTransform (Transformation|GetWorldLocation (.OutItem (Utilities|Array|Random (Variables|Default|GetComponents)))) "0, 0, 0" "0.300000,0.300000,0.300000") "Undefined" 0 0))

(event EventBeginPlay
  (Utilities|Time|SetTimerbyEvent (delegate Custom|SpawnEnemy) 1.0 true))

(event Collision|EventActorBeginOverlap
  (params (OtherActor :type Actor%20Object%20Reference)))

(event EventTick
  (params (DeltaSeconds :type Float%20%28single-precision%29)))

(fn ConstructionScript
  (bind _counter (Utilities|FlowControl|DoN (Variables|Default|GetCount) :!label _label)
    (:Exit
      (bind _returnvalue (AddComponent|AddSphereComponent false (Math|Conversions|ToTransform(Vector) (Math|Vector|MakeVector 0.0 (* _counter (Variables|Default|GetOffset)) 0.0))))
      (Utilities|Array|Add (Variables|Default|GetComponents) _returnvalue)
      (goto _label))))